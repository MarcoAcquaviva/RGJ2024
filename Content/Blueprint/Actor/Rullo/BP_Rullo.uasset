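; BP_Rullo is a conveyor belt actor that carries shopping items along its surface.
; Each Tick, it offsets every BP_ShoppingItemBase overlapping BoxCollision along the Arrow's forward vector, scaled by Velocity and delta time, without sweep or physics forces.
; The construction script puts a dynamic MI_Master instance on the mesh and passes Velocity to a scalar parameter, though that parameter's name is None.
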(event EventBeginPlay)

(event Collision|EventActorBeginOverlap
  (params (OtherActor :type Actor%20Object%20Reference)))

(event EventTick
  (params (DeltaSeconds :type Float%20%28single-precision%29))
  (for _array_element (Collision|GetOverlappingActors (Variables|Default|GetBoxCollision) "/Game/Blueprint/Actor/ShoppingItem/BP_ShoppingItemBase.BP_ShoppingItemBase_C" :!class /Script/Engine.PrimitiveComponent)
    (Transformation|AddActorWorldOffset _array_element (* (Math|Vector|GetForwardVector (Transformation|GetWorldRotation (Variables|Default|GetArrow))) (* DeltaSeconds (Variables|Default|GetVelocity))))))

(fn ConstructionScript
  (bind _returnvalue (Rendering|Material|CreateDynamicMaterialInstance "/Game/CustomAssets/Materials/MI_Master.MI_Master" "None" "None" :!class /Script/Engine.KismetMaterialLibrary))
  (Rendering|Material|SetScalarParameterValue _returnvalue "None" (Variables|Default|GetVelocity) :!class /Script/Engine.MaterialInstanceDynamic)
  (Rendering|Material|SetMaterial (Variables|Character|GetMesh) 0 _returnvalue))